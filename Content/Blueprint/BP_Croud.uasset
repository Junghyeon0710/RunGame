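; BP_Croud is a lethal obstacle actor that kills the third-person player character on contact.
; A hit event on its Block component casts the other actor to BP_ThirdPersonCharacter, stores the reference and calls Die on it.
; Other actors are ignored, and BeginPlay, overlap, Tick and the construction script add no logic of their own.
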(event `self.Block.OnComponentHit`
  (params (HitComponent :type "PrimitiveComponent Object Reference") (OtherActor :type "Actor Object Reference") (OtherComp :type "PrimitiveComponent Object Reference") (NormalImpulse :type "Vector Structure") (Hit :type "HitResult Structure (by ref)"))
  (bind _asbp_third_person_character (cast `/Game/ThirdPerson/Blueprints/BP_ThirdPersonCharacter` OtherActor))
  (bind _output_get (set `self.As BP Third Person Character` _asbp_third_person_character))
  (`RunCharacter.Die` _output_get))

(fn `UserConstructionScript`
  (`parent.UserConstructionScript`))