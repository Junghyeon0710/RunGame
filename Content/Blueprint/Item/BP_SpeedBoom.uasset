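; BP_SpeedBoom is a pickup item that gives BP_ThirdPersonCharacter a temporary speed boost.
; Overlapping its sphere sets the character's SpeedBoom flag, raises max walk speed and swaps the mesh material.
; Chained delays switch to a second material shortly before expiry, then restore hard-coded speed and body material and clear the flag.
; The actor destroys itself only after the boost ends, without hiding or disabling collision meanwhile.
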(event `self.Sphere.OnComponentBeginOverlap`
  (params (OverlappedComponent :type "PrimitiveComponent Object Reference") (OtherActor :type "Actor Object Reference") (OtherComp :type "PrimitiveComponent Object Reference") (OtherBodyIndex :type Integer) (bFromSweep :type Boolean) (SweepResult :type "HitResult Structure (by ref)"))
  (bind _asbp_third_person_character (cast `/Game/ThirdPerson/Blueprints/BP_ThirdPersonCharacter` OtherActor))
  (set `RunCharacter.bSpeedBoom` true _asbp_third_person_character)
  (bind _charactermovement (`Character.CharacterMovement` _asbp_third_person_character))
  (set `CharacterMovementComponent.MaxWalkSpeed` 3500.0 _charactermovement)
  (bind _mesh (`Character.Mesh` _asbp_third_person_character))
  (`PrimitiveComponent.SetMaterial` _mesh 0 "/AnimationSharing/AnimSharingRed.AnimSharingRed")
  (`KismetSystemLibrary.Delay` 4.0)
  (`PrimitiveComponent.SetMaterial` _mesh 0 "/AnimationSharing/AnimSharingRed1.AnimSharingRed1")
  (`KismetSystemLibrary.Delay` 1.0)
  (set `RunCharacter.bSpeedBoom` false _asbp_third_person_character)
  (set `CharacterMovementComponent.MaxWalkSpeed` 1500.0 _charactermovement)
  (`PrimitiveComponent.SetMaterial` _mesh 0 "/Game/Asset/Character/Ch03_Body.Ch03_Body")
  (`self.K2_DestroyActor`))

(event `커스텀이벤트`)

(fn `UserConstructionScript`)